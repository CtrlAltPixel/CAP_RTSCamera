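; RTS camera pawn that handles move, rotate, drag, screen-edge scroll and focus-on-actor events.
; Moves use movement input, with edge scrolling on world axes, while drag offsets the actor directly.
; Tick eases spring arm length toward ZoomValue and derives pitch from ZoomCurve over the normalized length.
; Zoom input only stores ZoomDirection; UpdateZoom runs at BeginPlay and multiplies it by zero, merely clamping ZoomValue.
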(event Custom|CameraMove
  (params (ActionValueX :type Float%20%28double-precision%29) (ActionValueY :type Float%20%28double-precision%29))
  ;[0.15 0.15 0.15 0.5] Comment
  (Pawn|Input|AddMovementInput (Transformation|GetActorForwardVector) ActionValueY false)
  (Pawn|Input|AddMovementInput (Transformation|GetActorRightVector) ActionValueX false))

(event Custom|CameraRotate
  (params (ActionValue :type Float%20%28double-precision%29))
  ;[0.15 0.15 0.15 0.5] Comment
  (Transformation|AddActorLocalRotation (Math|Rotator|MakeRotator 0.0 0.0 (* ActionValue 1.0)) false false))

(event Custom|CameraZoom
  (params (ActionValue :type Float%20%28double-precision%29))
  ;[0.15 0.15 0.15 0.5] Comment
  (Variables|Default|SetZoomDirection ActionValue))

(event Custom|CameraFocusActor
  (params (Actor :type Actor%20Object%20Reference))
  ;[0.15 0.15 0.15 0.5] Comment
  (Utilities|IsValid Actor
    (:Is%20Valid
      (Transformation|SetActorLocation (Transformation|GetActorLocation Actor) false false))))

(event Custom|CameraDrag
  (params (ActionValueX :type Float%20%28single-precision%29) (ActionValueY :type Float%20%28single-precision%29))
  ;[0.15 0.15 0.15 0.5] Comment
  (Transformation|AddActorWorldOffset (Math|Vector|MakeVector ActionValueX ActionValueY 0.0)))

(event EventBeginPlay
  ;[0.15 0.15 0.15 0.5] Comment
  (CallFunction|UpdateZoom))

(event EventTick
  (params (DeltaSeconds :type Float%20%28single-precision%29))
  (bind _zoomrange (Variables|Default|GetZoomRange))
  ;[0.15 0.15 0.15 0.5] Comment
  (bind _output_get (Variables|/Script/Engine.SpringArmComponent|SetTargetArmLength (Variables|Default|GetSpringArm) (Math|Interpolation|FInterpTo (Variables|/Script/Engine.SpringArmComponent|GetTargetArmLength (Variables|Default|GetSpringArm)) (Variables|Default|GetZoomValue) DeltaSeconds 3.0)))
  (Transformation|SetRelativeRotation (Variables|Default|GetSpringArm) (Math|Rotator|MakeRotator 0.0 (* (Math|Curves|GetFloatValue (Variables|Default|GetZoomCurve) (Math|Float|NormalizetoRange _output_get (.value (.lowerbound _zoomrange)) (.value (.upperbound _zoomrange)))) -62.0) 0.0) false false))

(event Input|MouseEvents|MouseX
  (params (AxisValue :type Float%20%28single-precision%29))
  (bind _returnvalue (Game|GetPlayerController 0))
  (bind _returnvalue_2 (Viewport|GetViewportSize))
  (bind _returnvalue_3 (Utilities|Time|GetWorldDeltaSeconds))
  (bind _edge_move_distance (Variables|Default|GetEdge%20Move%20Distance))
  (bind _locationx (Game|Player|GetMousePosition _returnvalue))
  (bind _returnvalue_4 (* _returnvalue_3 _edge_move_distance))
  (bind _returnvalue_5 (/ _locationx (.x _returnvalue_2)))
  ;[0.15 0.15 0.15 0.5] Comment
  (if (> _returnvalue_5 0.98)
    (Pawn|Input|AddMovementInput (Math|Vector|MakeVector 0.0 _returnvalue_4 0.0) 1.0 false)
    (elif (< _returnvalue_5 0.02)
      (Pawn|Input|AddMovementInput (Math|Vector|MakeVector 0.0 (* _returnvalue_4 -1.0) 0.0) 1.0 false))))

(event Input|MouseEvents|MouseY
  (params (AxisValue :type Float%20%28single-precision%29))
  (bind _returnvalue (Game|GetPlayerController 0))
  (bind _returnvalue_2 (Viewport|GetViewportSize))
  (bind _returnvalue_3 (Utilities|Time|GetWorldDeltaSeconds))
  (bind _edge_move_distance (Variables|Default|GetEdge%20Move%20Distance))
  (bind _locationy (Game|Player|GetMousePosition _returnvalue))
  (bind _returnvalue_4 (* _returnvalue_3 _edge_move_distance))
  (bind _returnvalue_5 (/ _locationy (.y _returnvalue_2)))
  ;[0.15 0.15 0.15 0.5] Comment
  (if (> _returnvalue_5 0.98)
    (Pawn|Input|AddMovementInput (Math|Vector|MakeVector (* _returnvalue_4 -1.0) 0.0 0.0) 1.0 false)
    (elif (< _returnvalue_5 0.02)
      (Pawn|Input|AddMovementInput (Math|Vector|MakeVector _returnvalue_4 0.0 0.0) 1.0 false))))

(fn ConstructionScript)

(fn UpdateZoom
  (bind _zoomrange (Variables|Default|GetZoomRange))
  (Variables|Default|SetZoomValue (Math|Float|Clamp(Float) (+ (Variables|Default|GetZoomValue) (* (Variables|Default|GetZoomDirection) 0.0)) (.value (.lowerbound _zoomrange)) (.value (.upperbound _zoomrange)))))

(fn DragtoMove
  (bind _previousmouselocation (Variables|Default|GetPreviousMouseLocation))
  (bind _newmouselocation (Variables|Default|GetNewMouseLocation))
  (bind _returnvalue (- _newmouselocation _previousmouselocation))
  (Pawn|Input|AddMovementInput (Math|Vector|MakeVector 0.0 (* (.x _returnvalue) -1.0) 0.0) 1.0 false)
  (Pawn|Input|AddMovementInput (Math|Vector|MakeVector (.y _returnvalue) 0.0 0.0) 1.0 false))