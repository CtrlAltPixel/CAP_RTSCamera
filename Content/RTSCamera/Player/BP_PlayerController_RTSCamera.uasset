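; Player controller for an RTS camera setup that turns Enhanced Input into camera commands and actor selection.
; Move, rotate, zoom, focus and drag-move inputs are forwarded to the possessed BP_Pawn_RTSCamera.
; Primary interact traces Pawns under the cursor and sends the selection to the HUD's character-selected widget.
; Pressing on no Pawn temporarily adds the drag-move mapping context, removed on release or cancel, so dragging and selecting share one input.
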(event Input|EnhancedActionEvents|EnhancedInputActionIA_PrimaryInteract
  (params (ActionValue :type Boolean) (ElapsedSeconds :type Float%20%28double-precision%29) (TriggeredSeconds :type Float%20%28double-precision%29) (InputAction :type Input%20Action%20Object%20Reference :default "/Game/RTSCamera/Input/Actions/IA_PrimaryInteract.IA_PrimaryInteract"))
  (:Triggered
    (CallFunction|UpdateSelectedActor (Variables|Default|GetAsClickedActor)))
  (:Started
    (bind _actor (CallFunction|GetActorUnderCursor))
    (bind _output_get (Variables|Default|SetAsClickedActor _actor))
    (Utilities|IsValid _output_get
      (:Is%20Valid
        _)
      (:Is%20Not%20Valid
        (Input|AddMappingContext (PlayerController|LocalPlayerSubsystems|GetEnhancedInputLocalPlayerSubsystem (Game|GetPlayerController 0)) "/Game/RTSCamera/Input/IMC_DragMove.IMC_DragMove" 0 "(bIgnoreAllPressedKeysUntilRelease=True,bForceImmediately=False,bNotifyUserSettings=False)")))
    (Variables|Default|SetAsSelectedActor 0))
  (:Canceled
    (Input|RemoveMappingContext (PlayerController|LocalPlayerSubsystems|GetEnhancedInputLocalPlayerSubsystem (Game|GetPlayerController 0)) "/Game/RTSCamera/Input/IMC_DragMove.IMC_DragMove" (Utilities|Struct|MakeModifyContextOptions true true false) :!label _label))
  (:Completed
    (goto _label)))

(event Input|EnhancedActionEvents|EnhancedInputActionIA_CameraMove
  (params (ActionValue :type Vector%202D%20Structure) (ElapsedSeconds :type Float%20%28double-precision%29) (TriggeredSeconds :type Float%20%28double-precision%29) (InputAction :type Input%20Action%20Object%20Reference :default "/Game/RTSCamera/Input/Actions/IA_CameraMove.IA_CameraMove"))
  (bind _as_bp_pawn_rtscamera (Variables|Default|GetAs%20BP%20Pawn%20RTSCamera)
    (:then
      (Default|CameraMove _as_bp_pawn_rtscamera (.x ActionValue) (.y ActionValue)))
    (:else)))

(event Input|EnhancedActionEvents|EnhancedInputActionIA_CameraRotate
  (params (ActionValue :type Float%20%28double-precision%29) (ElapsedSeconds :type Float%20%28double-precision%29) (TriggeredSeconds :type Float%20%28double-precision%29) (InputAction :type Input%20Action%20Object%20Reference :default "/Game/RTSCamera/Input/Actions/IA_CameraRotate.IA_CameraRotate"))
  (bind _as_bp_pawn_rtscamera (Variables|Default|GetAs%20BP%20Pawn%20RTSCamera)
    (:then
      (Default|CameraRotate _as_bp_pawn_rtscamera ActionValue))
    (:else)))

(event Input|EnhancedActionEvents|EnhancedInputActionIA_CameraZoom
  (params (ActionValue :type Float%20%28double-precision%29) (ElapsedSeconds :type Float%20%28double-precision%29) (TriggeredSeconds :type Float%20%28double-precision%29) (InputAction :type Input%20Action%20Object%20Reference :default "/Game/RTSCamera/Input/Actions/IA_CameraZoom.IA_CameraZoom"))
  (bind _as_bp_pawn_rtscamera (Variables|Default|GetAs%20BP%20Pawn%20RTSCamera)
    (:then
      (Default|CameraZoom _as_bp_pawn_rtscamera 0.0))
    (:else)))

(event Input|EnhancedActionEvents|EnhancedInputActionIA_CameraFocus
  (params (ActionValue :type Boolean) (ElapsedSeconds :type Float%20%28double-precision%29) (TriggeredSeconds :type Float%20%28double-precision%29) (InputAction :type Input%20Action%20Object%20Reference :default "/Game/RTSCamera/Input/Actions/IA_CameraFocus.IA_CameraFocus"))
  (bind _as_bp_pawn_rtscamera (Variables|Default|GetAs%20BP%20Pawn%20RTSCamera)
    (:then
      (Default|CameraFocusActor _as_bp_pawn_rtscamera))
    (:else)))

(event Input|EnhancedActionEvents|EnhancedInputActionIA_DragToMove
  (params (ActionValue :type Float%20%28double-precision%29) (ElapsedSeconds :type Float%20%28double-precision%29) (TriggeredSeconds :type Float%20%28double-precision%29) (InputAction :type Input%20Action%20Object%20Reference :default "/Game/RTSCamera/Input/Actions/IA_DragToMove.IA_DragToMove"))
  (:Started
    (bind _as_bp_pawn_rtscamera (Variables|Default|GetAs%20BP%20Pawn%20RTSCamera)
      (:then
        (bind _returnvalue (Class|WidgetLayoutLibrary|GetMousePositiononViewport))
        (Variables|/Game/RTSCamera/Camera/BP_Pawn_RTSCamera.BP_Pawn_RTSCamera_C|SetPreviousMouseLocation _as_bp_pawn_rtscamera _returnvalue))
      (:else)))
  (:Completed
    (bind _as_bp_pawn_rtscamera_2 (Variables|Default|GetAs%20BP%20Pawn%20RTSCamera)
      (:then
        (bind _returnvalue_2 (Class|WidgetLayoutLibrary|GetMousePositiononViewport))
        (bind _output_get (Variables|/Game/RTSCamera/Camera/BP_Pawn_RTSCamera.BP_Pawn_RTSCamera_C|SetNewMouseLocation _as_bp_pawn_rtscamera_2 _returnvalue_2))
        (Default|DragtoMove _as_bp_pawn_rtscamera_2)
        (Variables|/Game/RTSCamera/Camera/BP_Pawn_RTSCamera.BP_Pawn_RTSCamera_C|SetPreviousMouseLocation _as_bp_pawn_rtscamera_2 _output_get))
      (:else))))

(event EventBeginPlay
  (bind _returnvalue (Game|GetPlayerController 0))
  (bind _returnvalue_2 (PlayerController|LocalPlayerSubsystems|GetEnhancedInputLocalPlayerSubsystem _returnvalue))
  (if (Pawn|IsLocalPlayerController)
    (Input|AddMappingContext _returnvalue_2 "/Game/RTSCamera/Input/IMC_Camera.IMC_Camera" 0 "(bIgnoreAllPressedKeysUntilRelease=True,bForceImmediately=False,bNotifyUserSettings=False)")
    (Input|AddMappingContext _returnvalue_2 "/Game/RTSCamera/Input/IMC_Interact.IMC_Interact" 0 "(bIgnoreAllPressedKeysUntilRelease=True,bForceImmediately=False,bNotifyUserSettings=False)")
    (CallFunction|InitCasts)))

(fn ConstructionScript)

(fn InitCasts
  (bind _asbp_pawn_rtscamera (Utilities|Casting|CastToBP_Pawn_RTSCamera (Pawn|GetControlledPawn)))
  (Variables|Default|SetAs%20BP%20Pawn%20RTSCamera _asbp_pawn_rtscamera)
  (bind _asbp_hud_rtscamera (Utilities|Casting|CastToBP_HUD_RTSCamera (HUD|GetHUD)))
  (Variables|Default|SetAs%20BP%20HUD%20RTSCamera _asbp_hud_rtscamera))

(fn GetActorUnderCursor
  (return (.HitActor (Collision|BreakHitResult (.HitResult (Class|PlayerController|GetHitResultUnderCursorforObjects (Utilities|Array|MakeArray "ObjectTypeQuery3") true))))))

(fn UpdateSelectedActor
  (params (Actor :type Actor%20Object%20Reference))
  (Variables|Default|SetAsSelectedActor Actor)
  (bind _as_bp_hud_rtscamera (Variables|Default|GetAs%20BP%20HUD%20RTSCamera)
    (:then
      (Default|Update (Variables|/Game/RTSCamera/HUD/WB_HUD_RTSCamera.WB_HUD_RTSCamera_C|GetWB_Character_Selected (Variables|/Game/RTSCamera/HUD/BP_HUD_RTSCamera.BP_HUD_RTSCamera_C|GetAs%20WB_HUD_RTSCamera _as_bp_hud_rtscamera)) (Variables|Default|GetAsSelectedActor)))
    (:else)))